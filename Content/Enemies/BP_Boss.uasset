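; Boss enemy for the arena fight, with a timed entrance, difficulty-scaled health and damage, and its own health bar widget.
; Melee, running, teleport and special attacks play montages whose notifies toggle sword damage, lock yaw or spawn slash projectiles, then signal attack end.
; The teleport hides the boss and retries random reachable points near the player before resuming the uppercut.
; Damage is reduced during the charged special, and death notifies the tagged arena.
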(event `EyesVisibility`
  (bind _asbp_saant_game_mode (cast `/Game/Blueprints/BP_SaantGameMode` (`GameplayStatics.GetGameMode`)))
  (switch `/Game/Blueprints/Enum/DifficultyLevel_Enum` (`/Game/Blueprints/BP_SaantGameMode.Difficulty` _asbp_saant_game_mode)
    (:`NewEnumerator0`
      (`SceneComponent.SetVisibility` (`self.RightEye`) false false :!label _label)
      (`SceneComponent.SetVisibility` (`self.LeftEye_0`) false false))
    (:`NewEnumerator1`
      (goto _label))
    (:`NewEnumerator2`
      (`SceneComponent.SetVisibility` (`self.RightEye`) true false)
      (`SceneComponent.SetVisibility` (`self.LeftEye_0`) true false))))

(event `VisibilityTrick`
  (`SceneComponent.SetVisibility` (`self.Mesh`) false false)
  (`SceneComponent.SetVisibility` (`self.SwordHandle`) false false)
  (`SceneComponent.SetVisibility` (`self.GrinchHead`) false false)
  (`KismetSystemLibrary.Delay` 0.7)
  (`SceneComponent.SetVisibility` (`self.Mesh`) true false)
  (`SceneComponent.SetVisibility` (`self.SwordHandle`) true false)
  (`SceneComponent.SetVisibility` (`self.GrinchHead`) true false))

(event `self.ReceiveDestroyed`
  (`Widget.RemoveFromParent` (`self.BossWidget`)))

(event `self.ReceiveBeginPlay`
  (`parent.ReceiveBeginPlay`)
  (`|ExecutionSequence`
    (:`then_0`
      (`self.VisibilityTrick`)
      (`self.EyesVisibility`)
      (`self.SetDifficultyStats`)
      (bind _asaic_enemy (cast `/Game/AI/AIC_Enemy` (`self.GetController`)))
      (`/Engine/EditorBlueprintResources/StandardMacros.IsValid` _asaic_enemy
        (:`Is Valid`
          (`AIPerceptionComponent.SetSenseEnabled` (`/Game/AI/AIC_Enemy.AIPerception` _asaic_enemy) "/Script/AIModule.AISense_Sight" false)
          (`KismetSystemLibrary.Delay` 4.0)
          (bind _returnvalue (`|CreateWidget` "/Game/UI/GameUI/WBP_Boss.WBP_Boss_C"))
          (bind _output_get (set `self.BossWidget` _returnvalue))
          (`/Game/UI/GameUI/WBP_Boss.UpdateHealthBar` _output_get (`self.Health`) (`self.MaxHealth`))
          (`KismetSystemLibrary.Delay` 5.0)
          (`UserWidget.AddToViewport` _output_get 0))))
    (:`then_1`
      (set `self.CustomTimeDilation` 0.5)
      (`KismetSystemLibrary.Delay` 5.0)
      (set `self.CustomTimeDilation` 1.0))
    (:`then_2`
      (`KismetSystemLibrary.Delay` 6.0)
      (`SceneComponent.SetVisibility` (`self.SwordHandle`) false false)
      (`SceneComponent.SetVisibility` (`self.Sword`) true false))))

(event `self.ReceiveAnyDamage`
  (params (Damage :type "Float (single-precision)") (DamageType :type "DamageType Object Reference") (InstigatedBy :type "Controller Object Reference") (DamageCauser :type "Actor Object Reference"))
  (if (`self.bChargeSpecialAttack`)
    (`parent.ReceiveAnyDamage` (* Damage 0.2) DamageType InstigatedBy DamageCauser)
    (else
      (`parent.ReceiveAnyDamage` Damage DamageType InstigatedBy DamageCauser)))
  (`/Game/UI/GameUI/WBP_Boss.UpdateHealthBar` (`self.BossWidget`) (`self.Health`) (`self.MaxHealth`)))

(event `SetDifficultyStats`
  (bind _asbp_saant_game_mode (cast `/Game/Blueprints/BP_SaantGameMode` (`GameplayStatics.GetGameMode`)))
  (bind _difficulty (`/Game/Blueprints/BP_SaantGameMode.Difficulty` _asbp_saant_game_mode))
  (`KismetSystemLibrary.PrintString` (`KismetStringLibrary.Concat_StrStr` "Boss Difficulty: " (`|GetEnumeratorNameAsString` _difficulty)))
  (switch `/Game/Blueprints/Enum/DifficultyLevel_Enum` _difficulty
    (:`NewEnumerator0`
      (bind _output_get (set `self.MaxHealth` 2000.0))
      (set `self.Health` _output_get)
      (set `self.MinDefaultDamage` 30.0)
      (set `self.MaxDefaultDamage` 40.0)
      (set `self.SpecialAttackDamage` 30.0))
    (:`NewEnumerator1`
      (bind _output_get_2 (set `self.MaxHealth` 3000.0))
      (set `self.Health` _output_get_2)
      (set `self.MinDefaultDamage` 40.0)
      (set `self.MaxDefaultDamage` 50.0)
      (set `self.SpecialAttackDamage` 40.0))
    (:`NewEnumerator2`
      (bind _output_get_3 (set `self.MaxHealth` 4000.0))
      (set `self.Health` _output_get_3)
      (set `self.MinDefaultDamage` 50.0)
      (set `self.MaxDefaultDamage` 60.0)
      (set `self.SpecialAttackDamage` 50.0))))

(event `self.SwordBox.OnComponentBeginOverlap`
  (params (OverlappedComponent :type "PrimitiveComponent Object Reference") (OtherActor :type "Actor Object Reference") (OtherComp :type "PrimitiveComponent Object Reference") (OtherBodyIndex :type Integer) (bFromSweep :type Boolean) (SweepResult :type "HitResult Structure (by ref)"))
  (if (`self.bSwordAttack`)
    (bind _asbp_saant_character (cast `/Game/Blueprints/Character/BP_SaantCharacter` OtherActor))
    (`/Engine/EditorBlueprintResources/StandardMacros.IsValid` _asbp_saant_character
      (:`Is Valid`
        (`GameplayStatics.ApplyDamage` _asbp_saant_character (`KismetMathLibrary.Conv_IntToDouble` (`KismetMathLibrary.Round` (`KismetMathLibrary.RandomFloatInRange` (`self.MinDefaultDamage`) (`self.MaxDefaultDamage`)))) null self)
        (set `self.bSwordAttack` false)))))

(event `Entrance`
  (`|PlayMontage` (`self.Mesh`) "/Game/Enemies/Assets/Boss/Animations/Boss_Entrance_RM_Montage.Boss_Entrance_RM_Montage"
    (:`OnCompleted`
      _)
    (:`OnInterrupted`
      _))
  (`self.OnEntranceEnd`))

(event `/Game/AI/BPI_EnemyAI.DefaultAttack`
  (bind _mesh (`self.Mesh`))
  (switch `int` (`KismetMathLibrary.RandomIntegerInRange` 0 1)
    (:`0`
      (bind _notifyname (`|PlayMontage` _mesh "/Game/Enemies/Assets/Boss/Animations/Boss_Attack_SwingAndSlam_RM_Montage.Boss_Attack_SwingAndSlam_RM_Montage")
        (:`OnCompleted`
          (`self.OnAttackEnd` :!label _label_2)
          (set `self.bSwordAttack` false))
        (:`OnInterrupted`
          (goto _label_2))
        (:`OnNotifyBegin`
          (switch `name` _notifyname
            (:`Attack`
              (set `self.bSwordAttack` true))
            (:`AttackEnd`
              (set `self.bSwordAttack` false))))))
    (:`1`
      (bind _notifyname_2 (`|PlayMontage` _mesh "/Game/Enemies/Assets/Boss/Animations/Boss_Attack_HandAndSwordSwing_RM_Montage.Boss_Attack_HandAndSwordSwing_RM_Montage")
        (:`OnCompleted`
          (goto _label_2))
        (:`OnInterrupted`
          (goto _label_2))
        (:`OnNotifyBegin`
          (switch `name` _notifyname_2
            (:`Attack`
              (set `self.bSwordAttack` true))
            (:`AttackEnd`
              (set `self.bSwordAttack` false))))))))

(event `RunningAttack`
  (bind _mesh (`self.Mesh`))
  (switch `int` (`KismetMathLibrary.RandomIntegerInRange` 0 1)
    (:`0`
      (bind _notifyname (`|PlayMontage` _mesh "/Game/Enemies/Assets/Boss/Animations/Boss_Attack_Running_Simple_RM_Montage.Boss_Attack_Running_Simple_RM_Montage")
        (:`OnCompleted`
          (`self.OnAttackEnd` :!label _label_3)
          (set `self.bSwordAttack` false)
          (set `self.bUseControllerRotationYaw` true))
        (:`OnInterrupted`
          (goto _label_3))
        (:`OnNotifyBegin`
          (switch `name` _notifyname
            (:`Attack`
              (set `self.bSwordAttack` true))
            (:`AttackEnd`
              (set `self.bSwordAttack` false))
            (:`LockYaw`
              (set `self.bUseControllerRotationYaw` false))))))
    (:`1`
      (bind _notifyname_2 (`|PlayMontage` _mesh "/Game/Enemies/Assets/Boss/Animations/Boss_Attack_Running_WithAOEBlow_RM_Montage.Boss_Attack_Running_WithAOEBlow_RM_Montage")
        (:`OnCompleted`
          (goto _label_3))
        (:`OnInterrupted`
          (goto _label_3))
        (:`OnNotifyBegin`
          (switch `name` _notifyname_2
            (:`Attack`
              (set `self.bSwordAttack` true))
            (:`AttackEnd`
              (set `self.bSwordAttack` false))
            (:`LockYaw`
              (set `self.bUseControllerRotationYaw` false))))))))

(event `TeleportAttack`
  (bind _returnvalue (`self.K2_GetActorLocation`))
  (bind _notifyname (`|PlayMontage` (`self.Mesh`) "/Game/Enemies/Assets/Boss/Animations/Boss_Attack_Uppercut_RM_Montage.Boss_Attack_Uppercut_RM_Montage")
    (:`OnNotifyBegin`
      (switch `name` _notifyname
        (:`Teleport`
          (`NiagaraFunctionLibrary.SpawnSystemAtLocation` "/Game/Enemies/Assets/FX/Boss/NS_BossTeleport.NS_BossTeleport" (+ (`self.K2_GetActorLocation`) (* (`KismetMathLibrary.Vector_Forward`) 50.0)))
          (`KismetSystemLibrary.Delay` 0.8)
          (`self.SetActorHiddenInGame` true)
          (`PrimitiveComponent.SetCollisionEnabled` (`self.Mesh`) "NoCollision")
          (`AnimInstance.Montage_Stop` (`SkeletalMeshComponent.GetAnimInstance` (`self.Mesh`)) 0.0 "/Game/Enemies/Assets/Boss/Animations/Boss_Attack_Uppercut_RM_Montage.Boss_Attack_Uppercut_RM_Montage")
          (bind _returnvalue_2 (`self.K2_TeleportTo` (`NavigationSystemV1.K2_GetRandomReachablePointInRadius` (`self.K2_GetActorLocation` (`GameplayStatics.GetPlayerCharacter` 0)) 350.0 null null) :!label _label_4))
          (if _returnvalue_2
            (`NiagaraFunctionLibrary.SpawnSystemAtLocation` "/Game/Enemies/Assets/FX/Boss/NS_BossTeleport.NS_BossTeleport" _returnvalue)
            (`GameplayStatics.PlaySoundAtLocation` "/Game/Enemies/Assets/Boss/SFX/Cues/Grinch_Teleport_End_Cue.Grinch_Teleport_End_Cue" _returnvalue (struct) 1.0 1.0 0.0 null null null null)
            (`KismetSystemLibrary.Delay` 1.0)
            (`self.SetActorHiddenInGame` false)
            (`PrimitiveComponent.SetCollisionEnabled` (`self.Mesh`) "QueryAndPhysics")
            (bind _notifyname_2 (`|PlayMontage` (`self.Mesh`) "/Game/Enemies/Assets/Boss/Animations/Boss_Attack_Uppercut_RM_Montage.Boss_Attack_Uppercut_RM_Montage" 1.0 2.3)
              (:`OnCompleted`
                (`self.OnAttackEnd` :!label _label_5)
                (set `self.bSwordAttack` false))
              (:`OnInterrupted`
                (goto _label_5))
              (:`OnNotifyBegin`
                (switch `name` _notifyname_2
                  (:`AttackEnd`
                    (set `self.bSwordAttack` false)))))
            (else
              (goto _label_4))))
        (:`Attack`
          (set `self.bSwordAttack` true)
          (`KismetSystemLibrary.PrintString` "Hello"))))))

(event `SpecialAttack`
  (bind (_returnvalue_x _returnvalue_y _returnvalue_z) (`KismetMathLibrary.BreakVector` (`self.K2_GetActorLocation`)))
  (bind (_returnvalue_x_2 _returnvalue_y_2 _returnvalue_z_2) (`KismetMathLibrary.BreakVector` (`self.K2_GetActorLocation`)))
  (bind (_returnvalue_x_3 _returnvalue_y_3) (`KismetMathLibrary.BreakVector` (`SceneComponent.GetSocketLocation` (`self.Mesh`) "weapon")))
  (bind (_returnvalue_x_4 _returnvalue_y_4) (`KismetMathLibrary.BreakVector` (`SceneComponent.GetSocketLocation` (`self.Mesh`) "weapon")))
  (bind (_returnvalue_roll _returnvalue_pitch _returnvalue_yaw) (`KismetMathLibrary.BreakRotator` (`KismetMathLibrary.Conv_VectorToRotator` (`SceneComponent.GetForwardVector` (`self.CapsuleComponent`)))))
  (bind (_returnvalue_roll_2 _returnvalue_pitch_2 _returnvalue_yaw_2) (`KismetMathLibrary.BreakRotator` (`KismetMathLibrary.Conv_VectorToRotator` (`SceneComponent.GetForwardVector` (`self.CapsuleComponent`)))))
  (bind _notifyname (`|PlayMontage` (`self.Mesh`) "/Game/Enemies/Assets/Boss/Animations/Boss_Attack_ChargedComboAttack_RM_Montage.Boss_Attack_ChargedComboAttack_RM_Montage")
    (:`then`
      (set `self.bChargeSpecialAttack` true))
    (:`OnCompleted`
      (`self.OnAttackEnd` :!label _label_6)
      (set `self.bChargeSpecialAttack` false))
    (:`OnInterrupted`
      (goto _label_6))
    (:`OnNotifyBegin`
      (switch `name` _notifyname
        (:`SpecialHoriz`
          (bind _returnvalue (`|SpawnActorFromClass` "/Game/Enemies/BP_BossSpecialAttack.BP_BossSpecialAttack_C" (`KismetMathLibrary.MakeTransform` (`KismetMathLibrary.MakeVector` _returnvalue_x_3 _returnvalue_y_3 (- _returnvalue_z_2 150.0)) (`KismetMathLibrary.MakeRotator` 0.0 0.0 _returnvalue_yaw_2)) "AlwaysSpawn" "OverrideRootScale" null null))
          (set `/Game/Enemies/BP_BossSpecialAttack.Damage` (`self.SpecialAttackDamage`) _returnvalue))
        (:`SpecialVert`
          (bind _returnvalue_2 (`|SpawnActorFromClass` "/Game/Enemies/BP_BossSpecialAttack.BP_BossSpecialAttack_C" (`KismetMathLibrary.MakeTransform` (`KismetMathLibrary.MakeVector` _returnvalue_x_3 _returnvalue_y_3 _returnvalue_z_2) (`KismetMathLibrary.MakeRotator` 90.0 0.0 _returnvalue_yaw_2)) "AlwaysSpawn" "OverrideRootScale" null null))
          (set `/Game/Enemies/BP_BossSpecialAttack.Damage` (`self.SpecialAttackDamage`) _returnvalue_2))
        (:`SpecialDiag`
          (bind _returnvalue_3 (`|SpawnActorFromClass` "/Game/Enemies/BP_BossSpecialAttack.BP_BossSpecialAttack_C" (`KismetMathLibrary.MakeTransform` (`KismetMathLibrary.MakeVector` _returnvalue_x_4 _returnvalue_y_4 _returnvalue_z) (`KismetMathLibrary.MakeRotator` 45.0 0.0 _returnvalue_yaw)) "AlwaysSpawn" "OverrideRootScale" null null))
          (set `/Game/Enemies/BP_BossSpecialAttack.Damage` (`self.SpecialAttackDamage`) _returnvalue_3))))))

(event `/Game/AI/BPI_EnemyAI.DeathAction`
  (`parent.DeathAction`)
  (bind _outactors (`GameplayStatics.GetAllActorsOfClassWithTag` "/Game/Blueprints/ArenaSystem/BP_ArenaBoss.BP_ArenaBoss_C" "Arena3"))
  (for _array_element _outactors
    (message `/Game/Blueprints/ArenaSystem/BPI_Arena.EndArena` _array_element)))

(fn `SetMovementSpeed`
  (params (Speed :type "/Game/AI/Enums/EMovementSpeed Enum" :default "NewEnumerator0"))
  (returns (SpeedValue :type "Float (double-precision)"))
  (bind _output_get (set `CharacterMovementComponent.MaxWalkSpeed` (select `/Game/AI/Enums/EMovementSpeed` Speed :`NewEnumerator1` 400.0 :`NewEnumerator2` 500.0 :`NewEnumerator3` 1200.0) (`self.CharacterMovement`)))
  (return _output_get))

(fn `UserConstructionScript`
  (`parent.UserConstructionScript`))
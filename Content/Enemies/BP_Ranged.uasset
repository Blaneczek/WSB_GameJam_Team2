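; BP_Ranged is a ranged enemy character that fires projectiles at the player and can leap to a given destination.
; DefaultAttack plays a shotgun montage whose notify spawns a damaging BP_SaantProjectile aimed at the player, then signals attack end on completion or interruption.
; JumptoDestination launches the character along a suggested arc toward a point above the target location.
; SetMovementSpeed maps movement states from idle to sprinting onto the character's max walk speed.
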(event `/Game/AI/BPI_EnemyAI.DefaultAttack`
  (bind _notifyname (`|PlayMontage` (`self.Mesh`) "/Game/Enemies/Assets/DeerMan/Animations/DeerMan_Shotgun_Montage.DeerMan_Shotgun_Montage")
    (:`OnCompleted`
      (`self.OnAttackEnd` :!label _label))
    (:`OnInterrupted`
      (goto _label))
    (:`OnNotifyBegin`
      (switch `name` _notifyname
        (:`Fire`
          (bind _returnvalue (`|SpawnActorFromClass` "/Game/Enemies/BP_SaantProjectile.BP_SaantProjectile_C" (`KismetMathLibrary.MakeTransform` (- (`SceneComponent.K2_GetComponentLocation` (`self.projectileSpawn`)) (0.0 0.0 30.0)) (`KismetMathLibrary.FindLookAtRotation` (`self.K2_GetActorLocation`) (`self.K2_GetActorLocation` (`GameplayStatics.GetPlayerCharacter` 0)))) "AdjustIfPossibleButAlwaysSpawn" "MultiplyWithRoot" null null))
          (set `/Game/Enemies/BP_SaantProjectile.Damage` 2.0 _returnvalue))))))

(event `/Game/AI/BPI_EnemyAI.JumpToDestination`
  (params (Destination :type "Vector Structure"))
  (bind _outlaunchvelocity (`GameplayStatics.SuggestProjectileVelocity_CustomArc` (`self.K2_GetActorLocation`) (`KismetMathLibrary.MakeVector` (.x Destination) (.y Destination) (+ (.z Destination) 150.0))))
  (`self.LaunchCharacter` _outlaunchvelocity true true))

(fn `SetMovementSpeed`
  (params (Speed :type "/Game/AI/Enums/EMovementSpeed Enum" :default "NewEnumerator0"))
  (returns (SpeedValue :type "Float (double-precision)"))
  (bind _output_get (set `CharacterMovementComponent.MaxWalkSpeed` (select `/Game/AI/Enums/EMovementSpeed` Speed :`NewEnumerator1` 100.0 :`NewEnumerator2` 250.0 :`NewEnumerator3` 600.0 :!type "Float (single-precision)") (`self.CharacterMovement`)))
  (return _output_get))

(fn `UserConstructionScript`
  (`parent.UserConstructionScript`))
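; Trigger actor that plays a one-time boss introduction cutscene when the player character overlaps its collision.
; It disables input, hides the player UI, blends between two cameras with a shake and plays a Niagara spawn effect.
; After a delay it spawns BP_Boss at SpawnPoint, calls DisableScream and teleports the player to the trigger's location and rotation.
; Timed delays then blend the view back and restore input and UI.
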(event `self.CollisionComponent.OnComponentBeginOverlap`
  (params (OverlappedComponent :type "PrimitiveComponent Object Reference") (OtherActor :type "Actor Object Reference") (OtherComp :type "PrimitiveComponent Object Reference") (OtherBodyIndex :type Integer) (bFromSweep :type Boolean) (SweepResult :type "HitResult Structure (by ref)"))
  (bind _returnvalue (`GameplayStatics.GetPlayerController` 0))
  (bind _returnvalue_2 (`GameplayStatics.GetPlayerController` 0))
  (bind _asbp_saant_character (cast `/Game/Blueprints/Character/BP_SaantCharacter` OtherActor))
  (`/Engine/EditorBlueprintResources/StandardMacros.IsValid` _asbp_saant_character
    (:`Is Valid`
      (`/Engine/EditorBlueprintResources/StandardMacros.DoOnce` false
        (:`Completed`
          (`self.DisableInput` _asbp_saant_character _returnvalue_2)
          (bind _asbp_saant_game_mode (cast `/Game/Blueprints/BP_SaantGameMode` (`GameplayStatics.GetGameMode`)))
          (bind _player_ui_ref (`/Game/Blueprints/BP_SaantGameMode.Player_UI_Ref` _asbp_saant_game_mode))
          (`Widget.SetVisibility` _player_ui_ref "Hidden")
          (`PlayerController.SetViewTargetWithBlend` _returnvalue_2 (`self.CameraStart`) 0.0 "VTBlend_EaseIn" 0.0 false)
          (`PlayerController.SetViewTargetWithBlend` _returnvalue_2 (`self.CameraEnd`) 2.0 "VTBlend_Linear" 0.0 false)
          (`LegacyCameraShake.StartLegacyCameraShake` (`GameplayStatics.GetPlayerCameraManager` 0) "/Game/Enemies/BP_CameraShakeBoss.BP_CameraShakeBoss_C")
          (`NiagaraFunctionLibrary.SpawnSystemAtLocation` "/Game/Enemies/Assets/FX/Boss/NS_BossSpawn.NS_BossSpawn" (`self.K2_GetActorLocation` (`self.SpawnPoint`)))
          (`KismetSystemLibrary.Delay` 3.0)
          (bind _returnvalue_3 (`|SpawnActorFromClass` "/Game/Enemies/BP_Boss.BP_Boss_C" (`self.GetTransform` (`self.SpawnPoint`)) "AdjustIfPossibleButAlwaysSpawn" "MultiplyWithRoot" null "/Engine/BasicShapes/BasicShapeMaterial.BasicShapeMaterial" null))
          (`/Game/Enemies/BP_EnemyBase.DisableScream` _returnvalue_3)
          (`self.K2_SetActorLocation` _asbp_saant_character (`self.K2_GetActorLocation`) false false)
          (`Controller.SetControlRotation` _returnvalue (`self.K2_GetActorRotation`))
          (`KismetSystemLibrary.Delay` 2.0)
          (`PlayerController.SetViewTargetWithBlend` _returnvalue _asbp_saant_character 2.0 "VTBlend_Linear" 0.0 false)
          (`KismetSystemLibrary.Delay` 2.0)
          (`self.EnableInput` _asbp_saant_character _returnvalue)
          (`Widget.SetVisibility` _player_ui_ref "Visible"))))))

(fn `UserConstructionScript`)
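; Base enemy that scales health and vulnerability time by game mode level and adds itself to the alive count.
; Damage is reported to AI sense; low health opens a one-time, overlay-highlighted window where any hit kills, and fist hits trigger glory deaths.
; SetState forwards states to AIC_Enemy.
; DeathAction either bursts into Niagara and updates the enemy count, or plays a death montage before calling OnDeathEnd.
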(event `self.ReceiveBeginPlay`
  (`|ExecutionSequence`
    (:`then_0`
      (bind _asbp_saant_game_mode (cast `/Game/Blueprints/BP_SaantGameMode` (`GameplayStatics.GetGameMode`)))
      (`/Engine/EditorBlueprintResources/StandardMacros.IsValid` _asbp_saant_game_mode
        (:`Is Valid`
          (bind _output_get (set `self.As BP First Person Game Mode` _asbp_saant_game_mode))
          (switch `/Game/Blueprints/Enum/Eenemy_Lvl_Enum` (`/Game/Blueprints/BP_SaantGameMode.EnemyLVL` _output_get)
            (:`NewEnumerator0`
              (set `self.LvlVal` 1.0))
            (:`NewEnumerator1`
              (set `self.LvlVal` 2.0))
            (:`NewEnumerator2`
              (set `self.LvlVal` 3.0)))
          (`self.StatMath`)
          (`KismetSystemLibrary.PrintString` (`KismetStringLibrary.Concat_StrStr` "Helth:" " " (`KismetStringLibrary.Conv_DoubleToString` (`self.Health`)) " " "VulTime " "" (`KismetStringLibrary.Conv_DoubleToString` (`self.VulnerableStateTime`)))))
        (:`Is Not Valid`
          (`KismetSystemLibrary.PrintString` "game mode not valid in enemy base"))))
    (:`then_1`
      (bind _asbp_saant_character (cast `/Game/Blueprints/Character/BP_SaantCharacter` (`GameplayStatics.GetPlayerCharacter` 0)))
      (`/Engine/EditorBlueprintResources/StandardMacros.IsValid` _asbp_saant_character
        (:`Is Valid`
          (set `self.As BP First Person Character` _asbp_saant_character))
        (:`Is Not Valid`
          (`KismetSystemLibrary.PrintString` "player character not valid in enemy base"))))
    (:`then_2`
      (`/Engine/EditorBlueprintResources/StandardMacros.IncrementInt` (`/Game/Blueprints/BP_SaantGameMode.EnemiesAlive` (`self.As BP First Person Game Mode`))))))

(event `self.ReceiveAnyDamage`
  (params (Damage :type "Float (single-precision)") (DamageType :type "DamageType Object Reference") (InstigatedBy :type "Controller Object Reference") (DamageCauser :type "Actor Object Reference"))
  (bind _returnvalue (`GameplayStatics.GetPlayerCharacter` 0))
  (`AISense_Damage.ReportDamageEvent` self _returnvalue Damage (`self.K2_GetActorLocation` _returnvalue))
  (if (`self.Vulnerable?`)
    (set `self.Health` 0.0)
    (if (`/Game/Blueprints/Character/BP_SaantCharacter.AttackingWithFist?` (`self.As BP First Person Character`))
      (`GameplayStatics.PlaySound2D` "/Game/Music/SoundEffects/Doom_Eternal_-_Blood_Punch_Sound_Effect-YTConverter_app.Doom_Eternal_-_Blood_Punch_Sound_Effect-YTConverter_app" 1.0 1.0 0.0 null null)
      (set `self.GloryDeath` true))
    (`self.SetState` "NewEnumerator3")
    (else
      (`KismetSystemLibrary.PrintString` (`KismetStringLibrary.Conv_DoubleToString` Damage))
      (bind _output_get (set `self.Health` (- (`self.Health`) Damage)))
      (if (<= (/ _output_get 100.0) 0.1)
        (if (not (`self.AfterTimeOut?`))
          (`/Engine/EditorBlueprintResources/StandardMacros.DoOnce` false
            (:`Completed`
              (set `self.Vulnerable?` true)
              (`MeshComponent.SetOverlayMaterial` (`self.Mesh`) "/Game/Effects/VulnerableEnemy/M_Overlay.M_Overlay")
              (`self.VulnerableTimer`))))
        (if (<= _output_get 0.0)
          (`self.SetState` "NewEnumerator3"))))))

(event `VulnerableTimer`
  (`KismetSystemLibrary.Delay` (`self.VulnerableStateTime`))
  (`MeshComponent.SetOverlayMaterial` (`self.Mesh`) null)
  (set `self.Vulnerable?` false)
  (set `self.AfterTimeOut?` true))

(event `/Game/AI/BPI_EnemyAI.DeathAction`
  (bind _as_bp_first_person_game_mode (`self.As BP First Person Game Mode`))
  (if (`self.GloryDeath`)
    (`/Engine/EditorBlueprintResources/StandardMacros.DoOnce` false :!label _label
      (:`Completed`
        (set `self.GloryDeath` false)
        (`self.K2_DestroyActor`)
        (`NiagaraFunctionLibrary.SpawnSystemAtLocation` (`self.DeathNiagaraEffect`) (`self.K2_GetActorLocation`) (struct) (2.0 2.0 2.0))
        (`/Engine/EditorBlueprintResources/StandardMacros.DecrementInt` (`/Game/Blueprints/BP_SaantGameMode.EnemiesAlive` _as_bp_first_person_game_mode)
          (:`  `
            (`/Game/Blueprints/BP_SaantGameMode.EnemiesLeft` _as_bp_first_person_game_mode)))))
    (else
      (bind _notifyname (`|PlayMontage` (`self.Mesh`) (`self.DeathMontage`))
        (:`OnCompleted`
          _)
        (:`OnInterrupted`
          _)
        (:`OnNotifyBegin`
          (switch `name` _notifyname
            (:`Destroy`
              (goto _label)))))
      (`self.OnDeathEnd`))))

(fn `SetMovementSpeed`
  (params (Speed :type "/Game/AI/Enums/EMovementSpeed Enum" :default "NewEnumerator0"))
  (returns (SpeedValue :type "Float (double-precision)"))
  (return 0.0))

(fn `SetState`
  (params (NewParam :type "/Game/AI/Enums/EAIState Enum" :default "NewEnumerator0"))
  (bind _asaic_enemy (cast `/Game/AI/AIC_Enemy` (`self.GetController`)))
  (`/Engine/EditorBlueprintResources/StandardMacros.IsValid` _asaic_enemy
    (:`Is Valid`
      (switch `/Game/AI/Enums/EAIState` NewParam
        (:`NewEnumerator0`
          (`/Game/AI/AIC_Enemy.SetStateAsPassive` _asaic_enemy))
        (:`NewEnumerator1`
          (`/Game/AI/AIC_Enemy.SetStateAsAttacking` _asaic_enemy (`GameplayStatics.GetPlayerCharacter` 0)))
        (:`NewEnumerator3`
          (`/Game/AI/AIC_Enemy.SetStateAsDead` _asaic_enemy))))
    (:`Is Not Valid`
      (`KismetSystemLibrary.PrintString` "AI Controller not valid in enemy base"))))

(fn `StatMath`
  (if (== (`self.LvlVal`) 1.0)
    (return)
    (else
      (set `self.Health` (* (* (`self.Health`) (`self.LvlVal`)) 0.7))
      (set `self.VulnerableStateTime` (* (/ (`self.VulnerableStateTime`) (`self.LvlVal`)) 1.2))
      (return))))

(fn `UserConstructionScript`)
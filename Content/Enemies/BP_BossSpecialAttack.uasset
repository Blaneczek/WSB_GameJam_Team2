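; Boss special attack actor that travels forward along its local X axis at Speed, widening as it goes, and destroys itself after a fixed lifetime.
; Tick moves it without sweep and grows its Y scale by a fixed per-frame step up to a cap, so the widening depends on frame rate.
; The first Box overlap with BP_SaantCharacter applies Damage and spawns a blood splash Niagara effect, gated by DoOnce.
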(event `self.ReceiveBeginPlay`
  (`KismetSystemLibrary.Delay` 10.0)
  (`self.K2_DestroyActor`))

(event `self.ReceiveTick`
  (params (DeltaSeconds :type "Float (single-precision)"))
  (bind (_returnvalue_x _returnvalue_y) (`KismetMathLibrary.BreakVector` (`self.GetActorRelativeScale3D`)))
  (bind _returnvalue (+ _returnvalue_y 0.2))
  (`self.K2_AddActorLocalOffset` (* (* DeltaSeconds (`self.Speed`)) (1.0 0.0 0.0)))
  (if (<= _returnvalue 30.0)
    (`self.SetActorRelativeScale3D` (`KismetMathLibrary.MakeVector` 1.0 _returnvalue 1.0))))

(event `self.Box.OnComponentBeginOverlap`
  (params (OverlappedComponent :type "PrimitiveComponent Object Reference") (OtherActor :type "Actor Object Reference") (OtherComp :type "PrimitiveComponent Object Reference") (OtherBodyIndex :type Integer) (bFromSweep :type Boolean) (SweepResult :type "HitResult Structure (by ref)"))
  (bind _asbp_saant_character (cast `/Game/Blueprints/Character/BP_SaantCharacter` OtherActor))
  (`/Engine/EditorBlueprintResources/StandardMacros.IsValid` _asbp_saant_character
    (:`Is Valid`
      (`/Engine/EditorBlueprintResources/StandardMacros.DoOnce` false
        (:`Completed`
          (`GameplayStatics.ApplyDamage` _asbp_saant_character (`self.Damage`))
          (`NiagaraFunctionLibrary.SpawnSystemAtLocation` "/Game/Effects/BloodHitEffect/NS_Blood_Splash.NS_Blood_Splash" (`self.K2_GetActorLocation` _asbp_saant_character)))))))

(fn `UserConstructionScript`)
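; BP_SpawnEnemy is a trigger that spawns one random enemy when the player's BP_SaantCharacter overlaps its collision component.
; A DoOnce gate limits it to a single activation, which plays a Niagara spawn effect at SpawnPoint and waits briefly.
; It then randomly picks a slow melee, fast melee or ranged enemy class and spawns it at SpawnPoint's transform, adjusting for collisions but always spawning.
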(event `self.CollisionComponent.OnComponentBeginOverlap`
  (params (OverlappedComponent :type "PrimitiveComponent Object Reference") (OtherActor :type "Actor Object Reference") (OtherComp :type "PrimitiveComponent Object Reference") (OtherBodyIndex :type Integer) (bFromSweep :type Boolean) (SweepResult :type "HitResult Structure (by ref)"))
  (bind _returnvalue (`self.GetTransform` (`self.SpawnPoint`)))
  (bind _asbp_saant_character (cast `/Game/Blueprints/Character/BP_SaantCharacter` OtherActor))
  (`/Engine/EditorBlueprintResources/StandardMacros.IsValid` _asbp_saant_character
    (:`Is Valid`
      (`/Engine/EditorBlueprintResources/StandardMacros.DoOnce` false
        (:`Completed`
          (`NiagaraFunctionLibrary.SpawnSystemAtLocation` "/Game/Enemies/Assets/FX/Enemy/NS_EnemySpawn.NS_EnemySpawn" (`self.K2_GetActorLocation` (`self.SpawnPoint`)))
          (`KismetSystemLibrary.Delay` 2.0)
          (switch `int` (`KismetMathLibrary.RandomIntegerInRange` 0 2)
            (:`0`
              (`|SpawnActorFromClass` "/Game/Enemies/BP_SlowMelee.BP_SlowMelee_C" _returnvalue "AdjustIfPossibleButAlwaysSpawn" "MultiplyWithRoot" null "/Engine/BasicShapes/BasicShapeMaterial.BasicShapeMaterial" null))
            (:`1`
              (`|SpawnActorFromClass` "/Game/Enemies/BP_FastMelee1.BP_FastMelee1_C" _returnvalue "AdjustIfPossibleButAlwaysSpawn" "MultiplyWithRoot" null false "/Engine/BasicShapes/BasicShapeMaterial.BasicShapeMaterial" null))
            (:`2`
              (`|SpawnActorFromClass` "/Game/Enemies/BP_Ranged.BP_Ranged_C" _returnvalue "AdjustIfPossibleButAlwaysSpawn" "MultiplyWithRoot" null "/Engine/BasicShapes/BasicShapeMaterial.BasicShapeMaterial" null))))))))

(fn `UserConstructionScript`)
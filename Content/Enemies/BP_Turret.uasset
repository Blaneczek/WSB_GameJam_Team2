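; BP_Turret is a stationary, snowman-voiced enemy that shoots at the player.
; Attack plays a shot sound and spawns a BP_SaantProjectile at the ProjectileSpawn point, rotated from the turret's origin toward player 0.
; DeathAction plays a death sound, waits briefly, then spawns an explosion and destroys the actor.
; SetMovementSpeed ignores its input and returns zero.
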(event `Attack`
  (`GameplayStatics.SpawnSoundAtLocation` "/Game/Enemies/Assets/Turret/SFX/Snowman_Shoot_Cue.Snowman_Shoot_Cue" (`self.K2_GetActorLocation`) (struct) 1.0 1.0 0.0 null null)
  (`|SpawnActorFromClass` "/Game/Enemies/BP_SaantProjectile.BP_SaantProjectile_C" (`KismetMathLibrary.MakeTransform` (`SceneComponent.K2_GetComponentLocation` (`self.ProjectileSpawn`)) (`KismetMathLibrary.FindLookAtRotation` (`self.K2_GetActorLocation`) (`self.K2_GetActorLocation` (`GameplayStatics.GetPlayerCharacter` 0)))) "Undefined" "MultiplyWithRoot" null null))

(event `/Game/AI/BPI_EnemyAI.DeathAction`
  (bind _returnvalue (`self.K2_GetActorLocation`))
  (`GameplayStatics.SpawnSoundAtLocation` "/Game/Enemies/Assets/Turret/SFX/Snowman_Death_Cue.Snowman_Death_Cue" _returnvalue (struct) 1.0 1.0 0.0 null null)
  (`KismetSystemLibrary.Delay` 1.0)
  (`GameplayStatics.SpawnEmitterAtLocation` "/Game/StarterContent/Particles/P_Explosion.P_Explosion" _returnvalue)
  (`self.K2_DestroyActor`))

(fn `SetMovementSpeed`
  (params (Speed :type "/Game/AI/Enums/EMovementSpeed Enum" :default "NewEnumerator0"))
  (returns (SpeedValue :type "Float (double-precision)"))
  (return 0.0))

(fn `UserConstructionScript`
  (`parent.UserConstructionScript`))
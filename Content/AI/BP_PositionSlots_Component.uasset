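; Actor component that manages six position slots around its owner for AI, letting enemies claim the nearest free spot.
; Slots start unoccupied at the owner's location, and UpdateSlotsData overwrites their locations with supplied positions while keeping occupancy.
; CalculateBestSpot maps rounded distances from an enemy location to free slot indices and returns the minimum.
; OccupySlot and ReleaseSlot toggle reservations, and AnySlotAvailable reports whether any remain free.
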(event `self.ReceiveTick`
  (params (DeltaSeconds :type "Float (single-precision)")))

(event `self.ReceiveBeginPlay`
  (`self.InitializeSlotsData`))

(fn `AnySlotAvailable`
  (returns (`Any Slot` :type Boolean))
  (for _array_element (`self.Slots`)
    (if (not (break `/Game/AI/S_SlotsData` _array_element))
      (return true)))
  (return false))

(fn `CalculateBestSpot`
  (params (`Enemy Location` :type "Vector Structure"))
  (returns (Location :type "Vector Structure") (Index :type Integer) (AnySpot :type Boolean))
  (locals (Distances :type "Map of Integer to Integer"))
  (for (_array_element _array_index) (`self.Slots`)
    (if (not (break `/Game/AI/S_SlotsData` _array_element))
      (`BlueprintMapLibrary.Map_Add` (`local.Distances`) (`KismetMathLibrary.Round` (`KismetMathLibrary.Vector_Distance` `Enemy Location` (`.Location_4_B43F7FC1443EC47305650D9BA2FB2F11` (break `/Game/AI/S_SlotsData` _array_element)))) _array_index)))
  (bind _keys (`BlueprintMapLibrary.Map_Keys` (`local.Distances`)))
  (bind (_value _returnvalue) (`BlueprintMapLibrary.Map_Find` (`local.Distances`) (`.MinValue` (`KismetMathLibrary.MinOfIntArray` _keys))))
  (bind (_output_occupied _output_location) (break `/Game/AI/S_SlotsData` (`|GetArrayItem` (`self.Slots`) _value)))
  (return _output_location _value _returnvalue))

(fn `InitializeSlotsData`
  (bind _slots (`self.Slots`))
  (bind _returnvalue (`Actor.K2_GetActorLocation` (`self.GetOwner`)))
  (`|ExecutionSequence`
    (:`then_0`
      (`KismetArrayLibrary.Array_Add` _slots (make `/Game/AI/S_SlotsData` false _returnvalue)))
    (:`then_1`
      (`KismetArrayLibrary.Array_Add` _slots (make `/Game/AI/S_SlotsData` false _returnvalue)))
    (:`then_2`
      (`KismetArrayLibrary.Array_Add` _slots (make `/Game/AI/S_SlotsData` false _returnvalue)))
    (:`then_3`
      (`KismetArrayLibrary.Array_Add` _slots (make `/Game/AI/S_SlotsData` false _returnvalue)))
    (:`then_4`
      (`KismetArrayLibrary.Array_Add` _slots (make `/Game/AI/S_SlotsData` false _returnvalue)))
    (:`then_5`
      (`KismetArrayLibrary.Array_Add` _slots (make `/Game/AI/S_SlotsData` false _returnvalue)))))

(fn `OccupySlot`
  (params (Index :type Integer))
  (returns (SlotTaken :type Boolean))
  (bind _slots (`self.Slots`))
  (bind (_output_occupied _output_location) (break `/Game/AI/S_SlotsData` (`|GetArrayItem` _slots Index)))
  (if _output_occupied
    (return false)
    (else
      (`KismetArrayLibrary.Array_Set` _slots Index (make `/Game/AI/S_SlotsData` true _output_location))
      (return true))))

(fn `ReleaseSlot`
  (params (Index :type Integer))
  (bind _slots (`self.Slots`))
  (bind (_output_occupied _output_location) (break `/Game/AI/S_SlotsData` (`|GetArrayItem` _slots Index)))
  (`KismetArrayLibrary.Array_Set` _slots Index (make `/Game/AI/S_SlotsData` false _output_location)))

(fn `UpdateSlotsData`
  (params (Slot1 :type "Vector Structure") (Slot2 :type "Vector Structure") (Slot3 :type "Vector Structure") (Slot4 :type "Vector Structure") (Slot5 :type "Vector Structure") (Slot6 :type "Vector Structure"))
  (locals (NewLocalVar :type "/Game/AI/S_SlotsData Structure"))
  (bind _slots (`self.Slots`))
  (bind _slots_2 (`self.Slots`))
  (bind _output_occupied (break `/Game/AI/S_SlotsData` (`|GetArrayItem` _slots 5)))
  (bind _output_occupied_2 (break `/Game/AI/S_SlotsData` (`|GetArrayItem` _slots)))
  (bind _output_occupied_3 (break `/Game/AI/S_SlotsData` (`|GetArrayItem` _slots 1)))
  (bind _output_occupied_4 (break `/Game/AI/S_SlotsData` (`|GetArrayItem` _slots 2)))
  (bind _output_occupied_5 (break `/Game/AI/S_SlotsData` (`|GetArrayItem` _slots 3)))
  (bind _output_occupied_6 (break `/Game/AI/S_SlotsData` (`|GetArrayItem` _slots 4)))
  (`|ExecutionSequence`
    (:`then_0`
      (`KismetArrayLibrary.Array_Set` _slots_2 0 (make `/Game/AI/S_SlotsData` _output_occupied_2 Slot1)))
    (:`then_1`
      (`KismetArrayLibrary.Array_Set` _slots_2 1 (make `/Game/AI/S_SlotsData` _output_occupied_3 Slot2)))
    (:`then_2`
      (`KismetArrayLibrary.Array_Set` _slots_2 2 (make `/Game/AI/S_SlotsData` _output_occupied_4 Slot3)))
    (:`then_3`
      (`KismetArrayLibrary.Array_Set` _slots_2 3 (make `/Game/AI/S_SlotsData` _output_occupied_5 Slot4)))
    (:`then_4`
      (`KismetArrayLibrary.Array_Set` _slots_2 4 (make `/Game/AI/S_SlotsData` _output_occupied_6 Slot5)))
    (:`then_5`
      (`KismetArrayLibrary.Array_Set` _slots_2 5 (make `/Game/AI/S_SlotsData` _output_occupied Slot6)))))
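; BlockRocks_BP is a rock obstacle that the player can destroy, but only after coming near it.
; A Box overlap with a Player-tagged BP_SaantCharacter permanently arms it by setting CanBeDestroyed.
; Once armed, any damage plays a punch sound, spawns the NS_Blink_Fire Niagara effect at its location and destroys the actor.
; Overlay material calls for its meshes are present but disconnected.
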(event `self.ReceiveBeginPlay`)

(event `self.Box.OnComponentBeginOverlap`
  (params (OverlappedComponent :type "PrimitiveComponent Object Reference") (OtherActor :type "Actor Object Reference") (OtherComp :type "PrimitiveComponent Object Reference") (OtherBodyIndex :type Integer) (bFromSweep :type Boolean) (SweepResult :type "HitResult Structure (by ref)"))
  (if (`self.ActorHasTag` OtherActor "Player")
    (cast `/Game/Blueprints/Character/BP_SaantCharacter` OtherActor)
    (set `self.CanBeDestroyed?` true)))

(event `self.ReceiveAnyDamage`
  (params (Damage :type "Float (single-precision)") (DamageType :type "DamageType Object Reference") (InstigatedBy :type "Controller Object Reference") (DamageCauser :type "Actor Object Reference"))
  (if (`self.CanBeDestroyed?`)
    (`GameplayStatics.SpawnSound2D` "/Game/Music/SoundEffects/Doom_Eternal_-_Blood_Punch_Sound_Effect-YTConverter_app.Doom_Eternal_-_Blood_Punch_Sound_Effect-YTConverter_app" 1.0 1.0 0.0 null)
    (`NiagaraFunctionLibrary.SpawnSystemAtLocation` "/Game/BlinkAndDashVFX/VFX_Niagara/NS_Blink_Fire.NS_Blink_Fire" (`self.K2_GetActorLocation`))
    (`self.K2_DestroyActor`)))

(fn `UserConstructionScript`)
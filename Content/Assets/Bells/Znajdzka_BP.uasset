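; Collectible bell pickup that the player gathers by walking into its overlap sphere.
; On overlap with a Player-tagged BP_SaantCharacter, it increments the character's Finder count, plays a 2D pickup sound and spawns a Niagara blink effect.
; It then notifies BP_SaantGameMode through BellCollected and destroys itself, with failed character or game mode casts halting the sequence.
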(event `self.Sphere.OnComponentBeginOverlap`
  (params (OverlappedComponent :type "PrimitiveComponent Object Reference") (OtherActor :type "Actor Object Reference") (OtherComp :type "PrimitiveComponent Object Reference") (OtherBodyIndex :type Integer) (bFromSweep :type Boolean) (SweepResult :type "HitResult Structure (by ref)"))
  (if (`self.ActorHasTag` OtherActor "Player")
    (bind _asbp_saant_character (cast `/Game/Blueprints/Character/BP_SaantCharacter` OtherActor))
    (`/Engine/EditorBlueprintResources/StandardMacros.IncrementInt` (`/Game/Blueprints/Character/BP_SaantCharacter.Finder` _asbp_saant_character)
      (:`  `
        (`GameplayStatics.SpawnSound2D` "/Game/Music/SoundEffects/PickUpSFX.PickUpSFX" 1.0 1.0 0.0 null)
        (`NiagaraFunctionLibrary.SpawnSystemAtLocation` "/Game/BlinkAndDashVFX/VFX_Niagara/NS_Blink_Psionic.NS_Blink_Psionic" (`self.K2_GetActorLocation`))
        (bind _asbp_saant_game_mode (cast `/Game/Blueprints/BP_SaantGameMode` (`GameplayStatics.GetGameMode`)))
        (`/Engine/EditorBlueprintResources/StandardMacros.IsValid` _asbp_saant_game_mode
          (:`Is Valid`
            (`/Game/Blueprints/BP_SaantGameMode.BellCollected` _asbp_saant_game_mode))
          (:`Is Not Valid`
            _))
        (`self.K2_DestroyActor`)))))

(fn `UserConstructionScript`)
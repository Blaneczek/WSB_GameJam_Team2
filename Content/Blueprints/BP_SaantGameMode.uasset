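; Game mode for Saant that handles player save/load, the HUD, battle music and wave triggering.
; BeginPlay loads the save and adds Player_UI outside Loading_Level.
; SaveGame and LoadGame pass character ammo, health and transform plus level name through Saant_Sve_BP, though saved shotgun ammo restores into ShotgunAmmoClip.
; Tick ends fights and stops music when AliveEnemies hits zero, while EnemiesLeft separately checks EnemiesAlive to call CallSpawnWave.
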(event `self.ReceiveBeginPlay`
  (`self.LoadGame`)
  (bind _returnvalue (`GameplayStatics.GetCurrentLevelName` true))
  (if (not (`KismetStringLibrary.EqualEqual_StrStr` _returnvalue "Loading_Level"))
    (bind _returnvalue_2 (`|CreateWidget` "/Game/UI/GameUI/Player_UI.Player_UI_C"))
    (set `self.Player_UI_Ref` _returnvalue_2)
    (`UserWidget.AddToViewport` _returnvalue_2 0)))

(event `PlayBattleMusic`
  (if (not (`self.EnemiesDead`))
    (bind _returnvalue (`GameplayStatics.SpawnSound2D` "/Game/Music/All_I_Want_For_Christmas_Is_DOOM_v_2__BFG_Division_x_AIWFCIY_-YConverter_app.All_I_Want_For_Christmas_Is_DOOM_v_2__BFG_Division_x_AIWFCIY_-YConverter_app" 1.0 1.0 0.0 null))
    (set `self.2DSound` _returnvalue)))

(event `self.ReceiveTick`
  (params (DeltaSeconds :type "Float (single-precision)"))
  (bind _2dsound (`self.2DSound`))
  (if (`self.Fighting?`)
    (if (== (`self.AliveEnemies`) 0)
      (set `self.EnemiesDead` true)
      (set `self.Fighting?` false)
      (`/Engine/EditorBlueprintResources/StandardMacros.IsValid` _2dsound
        (:`Is Valid`
          (`AudioComponent.StopDelayed` _2dsound 1.0))))))

(event `EnemiesLeft`
  (if (== (`self.EnemiesAlive`) 0)
    (`self.SpawnWave`)))

(fn `GetPlayerData`
  (returns (AR_Ammo_Current :type Integer) (Shotgun_Ammo_Current :type Integer) (Health :type "Float (double-precision)") (CurrentPosition :type "Vector Structure") (CurrentRoation :type "Rotator Structure"))
  (bind _asbp_saant_character (cast `/Game/Blueprints/Character/BP_SaantCharacter` (`GameplayStatics.GetPlayerCharacter` 0)))
  (bind (_returnvalue_location _returnvalue_rotation) (`KismetMathLibrary.BreakTransform` (`self.GetTransform` _asbp_saant_character)))
  (return (`/Game/Blueprints/Character/BP_SaantCharacter.AR_Ammo_Current` _asbp_saant_character) (`/Game/Blueprints/Character/BP_SaantCharacter.Shotgun_Ammo_Current` _asbp_saant_character) (`/Game/Blueprints/Character/BP_SaantCharacter.Health` _asbp_saant_character) _returnvalue_location _returnvalue_rotation))

(fn `LoadGame`
  (bind _returnvalue (`GameplayStatics.DoesSaveGameExist` (`self.SaveName`)))
  (if _returnvalue
    (bind _returnvalue_2 (`GameplayStatics.LoadGameFromSlot` (`self.SaveName`)))
    (bind _assaant_sve_bp (cast `/Game/Blueprints/Saant_Sve_BP` _returnvalue_2))
    (bind (_ar_ammo_current _shotgun_ammo_current _health _currentlevel _current_position _current_rotation) (`/Game/Blueprints/Saant_Sve_BP.SetData` _assaant_sve_bp))
    (`self.SetPlayerData` _ar_ammo_current _shotgun_ammo_current _health _current_position _current_rotation)
    (set `self.Current Level` _currentlevel)
    (return)))

(fn `SaveGame`
  (bind _returnvalue (`GameplayStatics.DoesSaveGameExist` (`self.SaveName`)))
  (if _returnvalue
    (bind _returnvalue_2 (`GameplayStatics.LoadGameFromSlot` (`self.SaveName`)))
    (bind _assaant_sve_bp (cast `/Game/Blueprints/Saant_Sve_BP` _returnvalue_2))
    (set `self.As Saant Sve BP` _assaant_sve_bp)
    (else
      (bind _returnvalue_3 (`GameplayStatics.CreateSaveGameObject` "/Game/Blueprints/Saant_Sve_BP.Saant_Sve_BP_C"))
      (bind _output_get (set `self.As Saant Sve BP` _returnvalue_3))))
  (bind (_ar_ammo_current _shotgun_ammo_current _health _currentposition _currentroation) (`self.GetPlayerData`))
  (bind _returnvalue_4 (`GameplayStatics.GetCurrentLevelName` true))
  (`/Game/Blueprints/Saant_Sve_BP.SaveData` _output_get _ar_ammo_current _shotgun_ammo_current _health _returnvalue_4 _currentposition _currentroation)
  (`GameplayStatics.SaveGameToSlot` _output_get (`self.SaveName`))
  (return))

(fn `SetPlayerData`
  (params (ArAmmoCurrent :type Integer) (ShotgunAmmoCurrent :type Integer) (Heath :type "Float (double-precision)") (CurrentPosition :type "Vector Structure") (CurrentLocation :type "Rotator Structure"))
  (bind _asbp_saant_character (cast `/Game/Blueprints/Character/BP_SaantCharacter` (`GameplayStatics.GetPlayerCharacter` 0)))
  (set `/Game/Blueprints/Character/BP_SaantCharacter.AR_Ammo_Current` ArAmmoCurrent _asbp_saant_character)
  (set `/Game/Blueprints/Character/BP_SaantCharacter.Shotgun_Ammo_Clip` ShotgunAmmoCurrent _asbp_saant_character)
  (set `/Game/Blueprints/Character/BP_SaantCharacter.Health` Heath _asbp_saant_character)
  (`self.K2_SetActorLocation` _asbp_saant_character CurrentPosition false false)
  (`self.K2_SetActorRotation` _asbp_saant_character CurrentLocation false)
  (return))

(fn `UserConstructionScript`)
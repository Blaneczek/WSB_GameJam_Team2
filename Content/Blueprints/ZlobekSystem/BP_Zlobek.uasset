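; Post-arena upgrade cabin that rewards the player between timeline-animated entry and exit doors.
; EndArena opens the entry; a one-shot overlap shuts the player in and scales upgrade widget options by a multiplier favoring faster arena times from the GameMode.
; Choosing triggers LevelUP, which adds fixed speed, health and weapon damage bonuses, refills health and opens the exit.
; A second one-shot overlap seals the exit behind the player.
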(event `CheckArenaTime`
  (bind (_arenatimes_time1 _arenatimes_time2) (break `/Game/Blueprints/ZlobekSystem/FArenaTimes` (`self.ArenaTimes`)))
  (bind _output_get (set `self.ArenaTime` (`BlueprintMapLibrary.Map_Find` (`/Game/Blueprints/BP_SaantGameMode.ArenaTime` (`self.As BP Saant Game Mode`)) (`self.ArenaTag`))))
  (if (<= _output_get _arenatimes_time1)
    (set `self.Multiplier` 3.0)
    (elif (<= (`self.ArenaTime`) _arenatimes_time2)
      (set `self.Multiplier` 2.0)
      (else
        (set `self.Multiplier` 1.0)))))

(event `self.ReceiveBeginPlay`
  (bind _asbp_saant_game_mode (cast `/Game/Blueprints/BP_SaantGameMode` (`GameplayStatics.GetGameMode`)))
  (set `self.As BP Saant Game Mode` _asbp_saant_game_mode))

(event `/Game/Blueprints/ArenaSystem/BPI_Arena.EndArena`
  (bind (_direction _door_open) (`Timeline|OpenDoorIn`)
    (:`Update`
      (`SceneComponent.K2_SetRelativeRotation` (`self.DoorsIn`) (`KismetMathLibrary.MakeRotator` 0.0 0.0 (`KismetMathLibrary.Lerp` 0.0 120.0 _door_open)) false false))))

(event `self.Sphere.OnComponentBeginOverlap`
  (params (OverlappedComponent :type "PrimitiveComponent Object Reference") (OtherActor :type "Actor Object Reference") (OtherComp :type "PrimitiveComponent Object Reference") (OtherBodyIndex :type Integer) (bFromSweep :type Boolean) (SweepResult :type "HitResult Structure (by ref)"))
  (`/Engine/EditorBlueprintResources/StandardMacros.DoOnce` false
    (:`Completed`
      (bind _asbp_saant_character (cast `/Game/Blueprints/Character/BP_SaantCharacter` OtherActor))
      (set `self.As BP Saant Character` _asbp_saant_character)
      (`self.CheckArenaTime`)
      (`self.CloseCabin`)
      (`self.UpgradeChoice`))))

(event `CloseCabin`
  (`PrimitiveComponent.SetCollisionEnabled` (`self.BlockingIn`) "QueryAndPhysics")
  (bind (_direction _door_close) (`Timeline|CloseDoorIn`)
    (:`Update`
      (`SceneComponent.K2_SetRelativeRotation` (`self.DoorsIn`) (`KismetMathLibrary.MakeRotator` 0.0 0.0 (`KismetMathLibrary.Lerp` 120.0 0.0 _door_close)) false false))))

(event `UpgradeChoice`
  (bind _multiplier (`self.Multiplier`))
  (`KismetSystemLibrary.K2_ClearAndInvalidateTimerHandle` (`/Game/Blueprints/Character/BP_SaantCharacter.ARTimer` (`self.As BP Saant Character`)))
  (bind _returnvalue (`|CreateWidget` "/Game/Blueprints/ZlobekSystem/WBP_UpgradeChoice.WBP_UpgradeChoice_C" null (* _multiplier 20.0) (* _multiplier 2.0) (* _multiplier 3.0) (* _multiplier 20.0) (* _multiplier 2.0) (* _multiplier 3.0) (* _multiplier 2.0) (* _multiplier 5.0)))
  (`UserWidget.AddToViewport` _returnvalue 0)
  (add `/Game/Blueprints/ZlobekSystem/WBP_UpgradeChoice.UpgradeChosen` _returnvalue (delegate `LevelUP`)))

(event `LevelUP`
  (bind _as_bp_saant_character (`self.As BP Saant Character`))
  (bind _as_bp_saant_character_2 (`self.As BP Saant Character`))
  (bind _as_bp_saant_character_3 (`self.As BP Saant Character`))
  (bind _charactermovement (`Character.CharacterMovement` (`self.As BP Saant Character`)))
  (`KismetSystemLibrary.Delay` 0.5)
  (set `CharacterMovementComponent.MaxWalkSpeed` (+ (`CharacterMovementComponent.MaxWalkSpeed` _charactermovement) (`self.MovementSpeed`)) _charactermovement)
  (bind _output_get (set `/Game/Blueprints/Character/BP_SaantCharacter.MaxHealth` (+ (`/Game/Blueprints/Character/BP_SaantCharacter.MaxHealth` _as_bp_saant_character) (`self.HP`)) _as_bp_saant_character))
  (set `/Game/Blueprints/Character/BP_SaantCharacter.Health` _output_get _as_bp_saant_character)
  (set `/Game/Blueprints/Character/BP_SaantCharacter.AR Damage` (+ (`/Game/Blueprints/Character/BP_SaantCharacter.AR Damage` _as_bp_saant_character_2) (`self.ARDamage`)) _as_bp_saant_character_2)
  (set `/Game/Blueprints/Character/BP_SaantCharacter.ShotgunMaxDamage` (+ (`/Game/Blueprints/Character/BP_SaantCharacter.ShotgunMaxDamage` _as_bp_saant_character_3) (`self.ShotgunDamage`)) _as_bp_saant_character_3)
  (bind _returnvalue (`|CreateWidget` "/Game/Blueprints/ZlobekSystem/WBP_LevelUP.WBP_LevelUP_C"))
  (`UserWidget.AddToViewport` _returnvalue 0)
  (bind (_direction _door_close) (`Timeline|OpenDoorOut`)
    (:`Update`
      (`SceneComponent.K2_SetRelativeRotation` (`self.DoorsOut`) (`KismetMathLibrary.MakeRotator` 0.0 0.0 (`KismetMathLibrary.Lerp` 0.0 -120.0 _door_close)) false false))))

(event `self.BoxOut.OnComponentBeginOverlap`
  (params (OverlappedComponent :type "PrimitiveComponent Object Reference") (OtherActor :type "Actor Object Reference") (OtherComp :type "PrimitiveComponent Object Reference") (OtherBodyIndex :type Integer) (bFromSweep :type Boolean) (SweepResult :type "HitResult Structure (by ref)"))
  (`/Engine/EditorBlueprintResources/StandardMacros.DoOnce` false
    (:`Completed`
      (`PrimitiveComponent.SetCollisionEnabled` (`self.BlockingOut`) "QueryAndPhysics")
      (bind (_direction _door_close) (`Timeline|CloseDoorOut`)
        (:`Update`
          (`SceneComponent.K2_SetRelativeRotation` (`self.DoorsOut`) (`KismetMathLibrary.MakeRotator` 0.0 0.0 (`KismetMathLibrary.Lerp` -120.0 0.0 _door_close)) false false))))))

(fn `UserConstructionScript`)
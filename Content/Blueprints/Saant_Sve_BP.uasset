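; Save data Blueprint that holds the player's progress: health, ammo, weapon and movement upgrades, location, difficulty, bells, arena and run statistics, and tutorial completion.
; SaveData takes every value as an input and copies it into the matching member variable.
; Despite its name, SetData acts as the getter, returning all stored values at once.
; Neither function reads or writes a save slot; both only move data in and out of the object.
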(fn `SaveData`
  (params (AR_Ammo_Current :type Integer) (Shotgun_Ammo_Current :type Integer) (Health :type "Float (double-precision)") (CurrentLevel :type String) (Current_Position :type "Vector Structure") (Current_Rotation :type "Rotator Structure") (Difficulty :type "/Game/Blueprints/Enum/DifficultyLevel_Enum Enum" :default "NewEnumerator0") (MaxHealth :type "Float (double-precision)") (UpgradeHeal :type "Float (double-precision)") (Bells :type Integer) (ShotgunAmmoClip :type Integer) (ArAmmoClip :type Integer) (ShotgunDamage :type "Float (double-precision)") (ArDamage :type "Float (double-precision)") (Speed :type "Float (double-precision)") (EnemyLvl :type "/Game/Blueprints/Enum/Eenemy_Lvl_Enum Enum" :default "NewEnumerator0") (ArenaTimes :type "Map of Name to Float (double-precision)") (GameTime :type "Float (double-precision)") (EnemiesKilled :type Integer) (BellsCollected :type Integer) (DashForce :type Integer) (`TutorialCompleted?` :type Boolean))
  (set `self.AR_Ammo_Current` AR_Ammo_Current)
  (set `self.Shotgun_Ammo_Current` Shotgun_Ammo_Current)
  (set `self.Health` Health)
  (set `self.CurrentLevel` CurrentLevel)
  (set `self.Current_Position` Current_Position)
  (set `self.Current_Rotation` Current_Rotation)
  (set `self.Difficulty` Difficulty)
  (set `self.MaxHealth` MaxHealth)
  (set `self.UpgradeHeal` UpgradeHeal)
  (set `self.Bells` Bells)
  (set `self.ShotgunAmmoClip` ShotgunAmmoClip)
  (set `self.ArAmmoClip` ArAmmoClip)
  (set `self.ShotgunDamage` ShotgunDamage)
  (set `self.ArDamage` ArDamage)
  (set `self.Speed` Speed)
  (set `self.EnemyLvl` EnemyLvl)
  (set `self.ArenaTimes` ArenaTimes)
  (set `self.GameTime` GameTime)
  (set `self.EnemiesKilled` EnemiesKilled)
  (set `self.BellsColected` BellsCollected)
  (set `self.DashForce` DashForce)
  (set `self.TutorialCompleted?` `TutorialCompleted?`))

(fn `SetData`
  (returns (AR_Ammo_Current :type Integer) (Shotgun_Ammo_Current :type Integer) (Health :type "Float (double-precision)") (CurrentLevel :type String) (Current_Position :type "Vector Structure") (Current_Rotation :type "Rotator Structure") (Difficulty :type "/Game/Blueprints/Enum/DifficultyLevel_Enum Enum") (MaxHealth :type "Float (double-precision)") (UpgradeHeal :type "Float (double-precision)") (Bells :type Integer) (ShotgunAmmoClip :type Integer) (ArAmmoClip :type Integer) (ShotgunDamage :type "Float (double-precision)") (ArDamage :type "Float (double-precision)") (Speed :type "Float (double-precision)") (EnemyLvl :type "/Game/Blueprints/Enum/Eenemy_Lvl_Enum Enum") (ArenaTimes :type "Map of Name to Float (double-precision)") (GameTime :type "Float (double-precision)") (EnemiesKilled :type Integer) (BellsCollected :type Integer) (DashForce :type Integer) (`TutorialCompleted?` :type Boolean))
  (return (`self.AR_Ammo_Current`) (`self.Shotgun_Ammo_Current`) (`self.Health`) (`self.CurrentLevel`) (`self.Current_Position`) (`self.Current_Rotation`) (`self.Difficulty`) (`self.MaxHealth`) (`self.UpgradeHeal`) (`self.Bells`) (`self.ShotgunAmmoClip`) (`self.ArAmmoClip`) (`self.ShotgunDamage`) (`self.ArDamage`) (`self.Speed`) (`self.EnemyLvl`) (`self.ArenaTimes`) (`self.GameTime`) (`self.EnemiesKilled`) (`self.BellsColected`) (`self.DashForce`) (`self.TutorialCompleted?`)))
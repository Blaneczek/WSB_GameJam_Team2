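; Arena trigger that runs a series of enemy waves once the player character overlaps its box.
; It shows a waves widget with a timer, turns its spinning star red and binds SpawnWave to the game mode.
; Each wave uses a looping timer to spawn random enemies at reachable nearby points after a Niagara effect.
; When no waves remain, the star turns green, arena-tagged actors get an end message, and the spawner removes the widget and itself.
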(event `self.ReceiveBeginPlay`
  (bind _asbp_saant_game_mode (cast `/Game/Blueprints/BP_SaantGameMode` (`GameplayStatics.GetGameMode`)))
  (set `self.Game Mode` _asbp_saant_game_mode))

(event `self.ReceiveTick`
  (params (DeltaSeconds :type "Float (single-precision)"))
  (`SceneComponent.K2_AddRelativeRotation` (`self.Star`) (`KismetMathLibrary.MakeRotator` 0.0 0.0 (* DeltaSeconds 100.0)) false false))

(event `self.Box.OnComponentBeginOverlap`
  (params (OverlappedComponent :type "PrimitiveComponent Object Reference") (OtherActor :type "Actor Object Reference") (OtherComp :type "PrimitiveComponent Object Reference") (OtherBodyIndex :type Integer) (bFromSweep :type Boolean) (SweepResult :type "HitResult Structure (by ref)"))
  (bind _game_mode (`self.Game Mode`))
  (cast `/Game/Blueprints/Character/BP_SaantCharacter` OtherActor)
  (`/Engine/EditorBlueprintResources/StandardMacros.DoOnce` false
    (:`Completed`
      (bind _returnvalue (`|CreateWidget` "/Game/Blueprints/ArenaSystem/WBP_Waves.WBP_Waves_C" null (`self.NumberOfWaves`)))
      (bind _output_get (set `self.WavesWidget` _returnvalue))
      (`UserWidget.AddToViewport` _output_get 0)
      (set `/Game/Blueprints/BP_SaantGameMode.EnemiesAlive` 0 _game_mode)
      (add `/Game/Blueprints/BP_SaantGameMode.SpawnWave` _game_mode (delegate `SpawnWave`))
      (`self.SpawnWave`)
      (bind _returnvalue_2 (`PrimitiveComponent.CreateDynamicMaterialInstance` (`self.Star`) 0 "/Game/Assets/star_Inst.star_Inst" "None"))
      (bind _output_get_2 (set `self.DynamicMaterial` _returnvalue_2))
      (`MaterialInstanceDynamic.SetVectorParameterValue` _output_get_2 "Color" (make `LinearColor` 1.0 0.0 0.0 1.0))
      (bind _returnvalue_3 (`KismetSystemLibrary.K2_SetTimerDelegate` (delegate `CountTime`) 1.0 true))
      (set `self.TimerEvent` _returnvalue_3))))

(event `CountTime`
  (bind _time (`self.Time`))
  (`/Game/Blueprints/ArenaSystem/WBP_Waves.Update Time` (`self.WavesWidget`) _time)
  (`/Engine/EditorBlueprintResources/StandardMacros.IncrementFloat` _time))

(event `SpawnWave`
  (`/Game/Blueprints/ArenaSystem/WBP_Waves.Set Number of Waves Left` (`self.WavesWidget`) (`self.NumberOfWaves`))
  (set `self.SpawnedEnemy` 0)
  (if (> (`self.NumberOfWaves`) 0)
    (bind _returnvalue (`KismetSystemLibrary.K2_SetTimerDelegate` (delegate `SpawnEnemy`) 1.0 true))
    (else
      (`MaterialInstanceDynamic.SetVectorParameterValue` (`self.DynamicMaterial`) "Color" (make `LinearColor` 0.0 1.0 0.0 1.0))
      (`KismetSystemLibrary.K2_ClearAndInvalidateTimerHandle` (`self.TimerEvent`))
      (bind _outactors (`GameplayStatics.GetAllActorsWithTag` (`self.ArenaTag`)))
      (for _array_element _outactors
        (message `/Game/Blueprints/ArenaSystem/BPI_Arena.EndArena` _array_element)
        (`KismetSystemLibrary.Delay` 3.0 :!label _label)
        (`Widget.RemoveFromParent` (`self.WavesWidget`))
        (`self.K2_DestroyActor`))
      (goto _label))))

(event `SpawnEnemy`
  (bind _output_get (set `self.SpawnLocation` (`NavigationSystemV1.K2_GetRandomReachablePointInRadius` (`self.K2_GetActorLocation`) 1400.0 null null)))
  (`NiagaraFunctionLibrary.SpawnSystemAtLocation` "/Game/Enemies/Assets/FX/Enemy/NS_EnemySpawn.NS_EnemySpawn" _output_get)
  (`KismetSystemLibrary.Delay` 1.0)
  (bind _returnvalue (`|SpawnActorFromClass` (`|GetArrayItem` (`self.Enemies`) (`KismetMathLibrary.RandomIntegerInRange` 0 2)) (`KismetMathLibrary.MakeTransform` _output_get) "AdjustIfPossibleButAlwaysSpawn" "MultiplyWithRoot" null null))
  (bind _asbp_enemy_base (cast `/Game/Enemies/BP_EnemyBase` _returnvalue))
  (`/Game/Enemies/BP_EnemyBase.SetState` _asbp_enemy_base "NewEnumerator1")
  (`/Game/Enemies/BP_EnemyBase.DisableScream` _asbp_enemy_base)
  (bind _result (`/Engine/EditorBlueprintResources/StandardMacros.IncrementInt` (`self.SpawnedEnemy`))
    (:`  `
      (if (>= _result (`self.EnemiesPerWave`))
        (`KismetSystemLibrary.K2_ClearAndInvalidateTimerHandle` (stale `SpawnWave` _returnvalue))
        (`/Engine/EditorBlueprintResources/StandardMacros.DecrementInt` (`self.NumberOfWaves`))))))

(fn `UserConstructionScript`)
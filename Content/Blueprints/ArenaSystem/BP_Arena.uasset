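; Arena actor that seals and opens passages with timeline-animated spikes and blocking collision as an encounter starts and ends.
; The first BP_SaantCharacter overlap on TriggerIn runs StartArena, moving entry spikes and stairs and enabling BlockingIn.
; A one-shot BoxBlockingEnter overlap enables BlockingEnter and moves SpikesCloseEnter.
; EndArena, not called within this graph, disables BlockingOut and moves the exit spikes and stairs.
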(event `self.TriggerIn.OnComponentBeginOverlap`
  (params (OverlappedComponent :type "PrimitiveComponent Object Reference") (OtherActor :type "Actor Object Reference") (OtherComp :type "PrimitiveComponent Object Reference") (OtherBodyIndex :type Integer) (bFromSweep :type Boolean) (SweepResult :type "HitResult Structure (by ref)"))
  (`/Engine/EditorBlueprintResources/StandardMacros.DoOnce` false
    (:`Completed`
      (cast `/Game/Blueprints/Character/BP_SaantCharacter` OtherActor)
      (`self.StartArena`)
      (`PrimitiveComponent.SetCollisionEnabled` (`self.BlockingIn`) "QueryAndPhysics"))))

(event `StartArena`
  (bind _spikestairsin (`self.SpikeStairsIn`))
  (bind _spikesopenin (`self.SpikesOpenIn`))
  (bind _spikescloseenter (`self.SpikesCloseEnter`))
  (bind (_relativelocation_x _relativelocation_y) (`KismetMathLibrary.BreakVector` (`SceneComponent.RelativeLocation` _spikestairsin)))
  (bind (_relativelocation_x_2 _relativelocation_y_2) (`KismetMathLibrary.BreakVector` (`SceneComponent.RelativeLocation` _spikesopenin)))
  (bind (_relativelocation_x_3 _relativelocation_y_3) (`KismetMathLibrary.BreakVector` (`SceneComponent.RelativeLocation` _spikescloseenter)))
  (bind (_direction _newtrack_0) (`Timeline|StairsIn`)
    (:`Update`
      (`SceneComponent.K2_SetRelativeLocation` _spikestairsin (`KismetMathLibrary.MakeVector` _relativelocation_x _relativelocation_y (`KismetMathLibrary.Lerp` 1600.0 900.0 _newtrack_0)) false false)
      (`SceneComponent.K2_SetRelativeLocation` _spikesopenin (`KismetMathLibrary.MakeVector` _relativelocation_x_2 _relativelocation_y_2 (`KismetMathLibrary.Lerp` -700.0 76.0 _newtrack_0)) false false)
      (`SceneComponent.K2_SetRelativeLocation` _spikescloseenter (`KismetMathLibrary.MakeVector` _relativelocation_x_3 _relativelocation_y_3 (`KismetMathLibrary.Lerp` 1600.0 900.0 _newtrack_0)) false false))))

(event `/Game/Blueprints/ArenaSystem/BPI_Arena.EndArena`
  (bind _spikesopenout (`self.SpikesOpenOut`))
  (bind _spikestairsout (`self.SpikeStairsOut`))
  (bind (_relativelocation_x _relativelocation_y) (`KismetMathLibrary.BreakVector` (`SceneComponent.RelativeLocation` _spikesopenout)))
  (bind (_relativelocation_x_2 _relativelocation_y_2) (`KismetMathLibrary.BreakVector` (`SceneComponent.RelativeLocation` _spikestairsout)))
  (`PrimitiveComponent.SetCollisionEnabled` (`self.BlockingOut`) "NoCollision")
  (bind (_direction _newtrack_0) (`Timeline|Timeline`)
    (:`Update`
      (`SceneComponent.K2_SetRelativeLocation` _spikesopenout (`KismetMathLibrary.MakeVector` _relativelocation_x _relativelocation_y (`KismetMathLibrary.Lerp` 70.0 -730.0 _newtrack_0)) false false)
      (`SceneComponent.K2_SetRelativeLocation` _spikestairsout (`KismetMathLibrary.MakeVector` _relativelocation_x_2 _relativelocation_y_2 (`KismetMathLibrary.Lerp` 900.0 1600.0 _newtrack_0)) false false))))

(event `self.BoxBlockingEnter.OnComponentBeginOverlap`
  (params (OverlappedComponent :type "PrimitiveComponent Object Reference") (OtherActor :type "Actor Object Reference") (OtherComp :type "PrimitiveComponent Object Reference") (OtherBodyIndex :type Integer) (bFromSweep :type Boolean) (SweepResult :type "HitResult Structure (by ref)"))
  (bind _spikescloseenter (`self.SpikesCloseEnter`))
  (bind (_relativelocation_x _relativelocation_y) (`KismetMathLibrary.BreakVector` (`SceneComponent.RelativeLocation` _spikescloseenter)))
  (`/Engine/EditorBlueprintResources/StandardMacros.DoOnce` false
    (:`Completed`
      (`PrimitiveComponent.SetCollisionEnabled` (`self.BlockingEnter`) "QueryAndPhysics")
      (bind (_direction _newtrack_0) (`Timeline|Timeline_0`)
        (:`Update`
          (`SceneComponent.K2_SetRelativeLocation` _spikescloseenter (`KismetMathLibrary.MakeVector` _relativelocation_x _relativelocation_y (`KismetMathLibrary.Lerp` 900.0 1600.0 _newtrack_0)) false false))))))

(fn `UserConstructionScript`)
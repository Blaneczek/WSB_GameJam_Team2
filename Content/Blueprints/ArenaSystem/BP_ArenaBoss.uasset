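; Boss arena actor that seals the player in, spawns BP_Boss with an intro cutscene, and exposes EndArena to end the game after a delay.
; One-shot overlap triggers enable blocking collision and drive timelines that move the spike barriers.
; Arena start swaps background music for a battle track, then a delay-sequenced intro disables input, hides the UI, cuts between cameras with shake and Niagara effects, and restores control.
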(event `self.BoxBlockingEnter.OnComponentBeginOverlap`
  (params (OverlappedComponent :type "PrimitiveComponent Object Reference") (OtherActor :type "Actor Object Reference") (OtherComp :type "PrimitiveComponent Object Reference") (OtherBodyIndex :type Integer) (bFromSweep :type Boolean) (SweepResult :type "HitResult Structure (by ref)"))
  (bind _spikescloseenter (`self.SpikesCloseEnter`))
  (bind (_relativelocation_x _relativelocation_y) (`KismetMathLibrary.BreakVector` (`SceneComponent.RelativeLocation` _spikescloseenter)))
  (`/Engine/EditorBlueprintResources/StandardMacros.DoOnce` false
    (:`Completed`
      (`PrimitiveComponent.SetCollisionEnabled` (`self.BlockingEnter`) "QueryAndPhysics")
      (bind (_direction _newtrack_0) (`Timeline|Timeline_1`)
        (:`Update`
          (`SceneComponent.K2_SetRelativeLocation` _spikescloseenter (`KismetMathLibrary.MakeVector` _relativelocation_x _relativelocation_y (`KismetMathLibrary.Lerp` 900.0 1600.0 _newtrack_0)) false false))))))

(event `self.TriggerIn.OnComponentBeginOverlap`
  (params (OverlappedComponent :type "PrimitiveComponent Object Reference") (OtherActor :type "Actor Object Reference") (OtherComp :type "PrimitiveComponent Object Reference") (OtherBodyIndex :type Integer) (bFromSweep :type Boolean) (SweepResult :type "HitResult Structure (by ref)"))
  (`/Engine/EditorBlueprintResources/StandardMacros.DoOnce` false
    (:`Completed`
      (bind _asbp_saant_character (cast `/Game/Blueprints/Character/BP_SaantCharacter` OtherActor))
      (set `self.As BP Saant Character` _asbp_saant_character)
      (`self.StartArena`)
      (`PrimitiveComponent.SetCollisionEnabled` (`self.BlockingIn`) "QueryAndPhysics")
      (`self.SpawnBoss`))))

(event `StartArena`
  (bind _spikestairsin (`self.SpikeStairsIn`))
  (bind _spikesopenin (`self.SpikesOpenIn`))
  (bind _spikescloseenter (`self.SpikesCloseEnter`))
  (bind (_relativelocation_x _relativelocation_y) (`KismetMathLibrary.BreakVector` (`SceneComponent.RelativeLocation` _spikestairsin)))
  (bind (_relativelocation_x_2 _relativelocation_y_2) (`KismetMathLibrary.BreakVector` (`SceneComponent.RelativeLocation` _spikesopenin)))
  (bind (_relativelocation_x_3 _relativelocation_y_3) (`KismetMathLibrary.BreakVector` (`SceneComponent.RelativeLocation` _spikescloseenter)))
  (`|ExecutionSequence`
    (:`then_0`
      (bind (_direction _newtrack_0) (`Timeline|Timeline`)
        (:`Update`
          (`SceneComponent.K2_SetRelativeLocation` _spikestairsin (`KismetMathLibrary.MakeVector` _relativelocation_x _relativelocation_y (`KismetMathLibrary.Lerp` 1600.0 900.0 _newtrack_0)) false false)
          (`SceneComponent.K2_SetRelativeLocation` _spikesopenin (`KismetMathLibrary.MakeVector` _relativelocation_x_2 _relativelocation_y_2 (`KismetMathLibrary.Lerp` -700.0 76.0 _newtrack_0)) false false)
          (`SceneComponent.K2_SetRelativeLocation` _spikescloseenter (`KismetMathLibrary.MakeVector` _relativelocation_x_3 _relativelocation_y_3 (`KismetMathLibrary.Lerp` 1600.0 900.0 _newtrack_0)) false false))))
    (:`then_1`
      (bind _asbp_saant_game_mode (cast `/Game/Blueprints/BP_SaantGameMode` (`GameplayStatics.GetGameMode`)))
      (`/Game/Blueprints/BP_SaantGameMode.StopBackgroundMusic` _asbp_saant_game_mode)
      (`GameplayStatics.SpawnSound2D` "/Game/Music/DOOM_Eternal_OST_Gladiator.DOOM_Eternal_OST_Gladiator" 0.3 1.0 0.0 null)
      (set `/Game/Blueprints/BP_SaantGameMode.ArenaBattleSound` null _asbp_saant_game_mode))))

(event `SpawnBoss`
  (bind _returnvalue (`GameplayStatics.GetPlayerController` 0))
  (bind _returnvalue_2 (`GameplayStatics.GetPlayerController` 0))
  (bind _returnvalue_3 (`GameplayStatics.GetPlayerController` 0))
  (bind _triggerin (`self.TriggerIn`))
  (bind _as_bp_saant_character (`self.As BP Saant Character`))
  (`KismetSystemLibrary.PrintString` "spawnboss")
  (`self.DisableInput` _as_bp_saant_character _returnvalue_2)
  (bind _asbp_saant_game_mode (cast `/Game/Blueprints/BP_SaantGameMode` (`GameplayStatics.GetGameMode`)))
  (set `self.As BP Saant Game Mode` _asbp_saant_game_mode)
  (bind _player_ui_ref (`/Game/Blueprints/BP_SaantGameMode.Player_UI_Ref` _asbp_saant_game_mode))
  (`Widget.SetVisibility` _player_ui_ref "Hidden")
  (`PlayerController.SetViewTargetWithBlend` _returnvalue_2 (`self.CameraPlayer`) 0.0 "VTBlend_EaseIn" 0.0 false)
  (`PlayerController.SetViewTargetWithBlend` _returnvalue_2 (`self.Camera1`) 2.0 "VTBlend_Linear" 0.0 false)
  (`LegacyCameraShake.StartLegacyCameraShake` (`GameplayStatics.GetPlayerCameraManager` 0) "/Game/Blueprints/ArenaSystem/BP_CameraShakeBoss.BP_CameraShakeBoss_C")
  (`NiagaraFunctionLibrary.SpawnSystemAtLocation` "/Game/Enemies/Assets/FX/Boss/NS_BossSpawn.NS_BossSpawn" (`self.K2_GetActorLocation` (`self.SpawnPoint`)))
  (`KismetSystemLibrary.Delay` 3.0)
  (bind _returnvalue_4 (`|SpawnActorFromClass` "/Game/Enemies/BP_Boss.BP_Boss_C" (`self.GetTransform` (`self.SpawnPoint`)) "AdjustIfPossibleButAlwaysSpawn" "MultiplyWithRoot" null "/Engine/BasicShapes/BasicShapeMaterial.BasicShapeMaterial" null))
  (`/Game/Enemies/BP_EnemyBase.SetState` _returnvalue_4 "NewEnumerator0")
  (`/Game/Enemies/BP_EnemyBase.DisableScream` _returnvalue_4)
  (`self.K2_SetActorLocation` _as_bp_saant_character (- (`SceneComponent.K2_GetComponentLocation` _triggerin) (0.0 0.0 200.0)) false false)
  (`Controller.SetControlRotation` _returnvalue (`SceneComponent.K2_GetComponentRotation` _triggerin))
  (`KismetSystemLibrary.Delay` 3.0)
  ;[0 0 0] Camera System
  (`PlayerController.SetViewTargetWithBlend` _returnvalue_3 (`self.Camera2`) 0.0 "VTBlend_Linear" 0.0 false)
  (`KismetSystemLibrary.Delay` 2.0)
  (`PlayerController.SetViewTargetWithBlend` _returnvalue_3 (`self.Camera3`) 0.0 "VTBlend_Linear" 0.0 false)
  (`KismetSystemLibrary.Delay` 2.0)
  (`PlayerController.SetViewTargetWithBlend` _returnvalue_3 (`self.Camera1`) 0.0 "VTBlend_Linear" 0.0 false)
  (`KismetSystemLibrary.Delay` 2.0)
  (`PlayerController.SetViewTargetWithBlend` _returnvalue _as_bp_saant_character 4.0 "VTBlend_Linear" 0.0 false)
  (`KismetSystemLibrary.Delay` 4.5)
  (`self.EnableInput` _as_bp_saant_character _returnvalue)
  (`Widget.SetVisibility` _player_ui_ref "Visible"))

(event `/Game/Blueprints/ArenaSystem/BPI_Arena.EndArena`
  (`KismetSystemLibrary.Delay` 3.0)
  (`/Game/Blueprints/BP_SaantGameMode.EndGame` (`self.As BP Saant Game Mode`)))

(fn `UserConstructionScript`)
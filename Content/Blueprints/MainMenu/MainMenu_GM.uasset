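; Main menu game mode that shows the main menu UI with mouse cursor and UI-only input, and plays menu music on start.
; It loads user video settings and the saved level, then applies display settings plus Master, Music and SFX volumes through a sound mix override.
; It syncs readable labels to a video settings widget.
; SaveGame writes either a fresh starting save or the existing progress with updated difficulty.
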(event `self.ReceiveBeginPlay`
  (bind _returnvalue (`GameplayStatics.GetPlayerController` 0))
  (`self.LoadGameSettings`)
  (`self.LoadGame`)
  (bind _returnvalue_2 (`|CreateWidget` "/Game/UI/MainMenu/MainMenu_Main_UI.MainMenu_Main_UI_C"))
  (`UserWidget.AddToViewport` _returnvalue_2 0)
  (set `PlayerController.bShowMouseCursor` true _returnvalue)
  (`WidgetBlueprintLibrary.SetInputMode_UIOnlyEx` _returnvalue _returnvalue_2)
  (`GameplayStatics.PlaySound2D` "/Game/Music/Doom_Eternal_-_Main_Theme__Official_Version_-YConverter_app.Doom_Eternal_-_Main_Theme__Official_Version_-YConverter_app" 1.0 1.0 0.0 null null)
  (`GameplayStatics.PlaySound2D` "/Game/Music/SoundEffects/Christmas_Bells-Sound_Effect-YConverter_app.Christmas_Bells-Sound_Effect-YConverter_app" 1.0 1.0 0.0 null null))

(event `ApplySettings`
  (bind _returnvalue (`GameUserSettings.GetGameUserSettings`))
  (`GameUserSettings.SetFullscreenMode` _returnvalue (`self.WindowMode`))
  (`GameUserSettings.SetOverallScalabilityLevel` _returnvalue (`self.GraphicIndex`))
  (`GameUserSettings.SetVSyncEnabled` _returnvalue (`self.VSync`))
  (`GameUserSettings.SetScreenResolution` _returnvalue (`self.Resolution`))
  (`GameUserSettings.ApplySettings` _returnvalue true)
  (`GameplayStatics.SetSoundMixClassOverride` "/Game/Blueprints/MainMenu/Saant_SoundMix.Saant_SoundMix" "/Engine/EngineSounds/Master.Master" (`self.MasterVolumeValue`))
  (`GameplayStatics.SetSoundMixClassOverride` "/Game/Blueprints/MainMenu/Saant_SoundMix.Saant_SoundMix" "/Engine/EngineSounds/Music.Music" (`self.MusicVolumeValue`))
  (`GameplayStatics.SetSoundMixClassOverride` "/Game/Blueprints/MainMenu/Saant_SoundMix.Saant_SoundMix" "/Engine/EngineSounds/SFX.SFX" (`self.SFXVolumeValue`))
  (`GameplayStatics.PushSoundMixModifier` "/Game/Blueprints/MainMenu/Saant_SoundMix.Saant_SoundMix"))

(event `AddToViewportVideoSettingsWidget`
  (`UserWidget.AddToViewport` (`self.VideoUI Ref`) 0))

(event `DestroyVideoSettingsWidget`
  (`Widget.RemoveFromParent` (`self.VideoUI Ref`)))

(event `UpdateSettingsStats`
  (bind _videoui_ref (`self.VideoUI Ref`))
  (bind (_resolution_x _resolution_y) (break `IntPoint` (`self.Resolution`)))
  (set `/Game/UI/MainMenu/Settings/Video_UI.Resolution X` _resolution_x _videoui_ref)
  (set `/Game/UI/MainMenu/Settings/Video_UI.Resolution Y` _resolution_y _videoui_ref)
  (switch `EWindowMode` (`self.WindowMode`)
    (:`Fullscreen`
      (set `/Game/UI/MainMenu/Settings/Video_UI.WindowMode` "FULLSCREEN" _videoui_ref))
    (:`WindowedFullscreen`
      (set `/Game/UI/MainMenu/Settings/Video_UI.WindowMode` "WINDOWED FULLSCREEN" _videoui_ref))
    (:`Windowed`
      (set `/Game/UI/MainMenu/Settings/Video_UI.WindowMode` "WINDOWED" _videoui_ref)))
  (switch `int` (`self.GraphicIndex`)
    (:`0`
      (set `/Game/UI/MainMenu/Settings/Video_UI.GraphicModeText` "Potato PC" _videoui_ref))
    (:`1`
      (set `/Game/UI/MainMenu/Settings/Video_UI.GraphicModeText` "Kinda Good" _videoui_ref))
    (:`2`
      (set `/Game/UI/MainMenu/Settings/Video_UI.GraphicModeText` "Good" _videoui_ref))
    (:`3`
      (set `/Game/UI/MainMenu/Settings/Video_UI.GraphicModeText` "Avarage" _videoui_ref))
    (:`4`
      (set `/Game/UI/MainMenu/Settings/Video_UI.GraphicModeText` "DAMN" _videoui_ref))))

(fn `LoadGame`
  (bind _returnvalue (`GameplayStatics.DoesSaveGameExist` (`self.SaveName`)))
  (if _returnvalue
    (bind _returnvalue_2 (`GameplayStatics.LoadGameFromSlot` (`self.SaveName`)))
    (bind _assaant_sve_bp (cast `/Game/Blueprints/Saant_Sve_BP` _returnvalue_2))
    (bind (_ar_ammo_current _shotgun_ammo_current _health _currentlevel) (`/Game/Blueprints/Saant_Sve_BP.SetData` _assaant_sve_bp))
    (set `self.LevelToOpen` _currentlevel)))

(fn `LoadGameSettings`
  (bind _returnvalue (`GameUserSettings.GetGameUserSettings`))
  (`GameUserSettings.LoadSettings` _returnvalue false)
  (set `self.WindowMode` (`GameUserSettings.GetFullscreenMode` _returnvalue))
  (set `self.GraphicIndex` (`GameUserSettings.GetOverallScalabilityLevel` _returnvalue))
  (set `self.VSync` (`GameUserSettings.IsVSyncEnabled` _returnvalue))
  (set `self.Resolution` (`GameUserSettings.GetScreenResolution` _returnvalue)))

(fn `SaveGame`
  (params (NewSave :type Boolean))
  (bind _returnvalue (`GameplayStatics.DoesSaveGameExist` (`self.SaveName`)))
  (if _returnvalue
    (bind _returnvalue_2 (`GameplayStatics.LoadGameFromSlot` (`self.SaveName`)))
    (bind _assaant_sve_bp (cast `/Game/Blueprints/Saant_Sve_BP` _returnvalue_2))
    (set `self.As Saant Sve BP` _assaant_sve_bp)
    (else
      (bind _returnvalue_3 (`GameplayStatics.CreateSaveGameObject` "/Game/Blueprints/Saant_Sve_BP.Saant_Sve_BP_C"))
      (bind _output_get (set `self.As Saant Sve BP` _returnvalue_3))))
  (if NewSave
    (`/Game/Blueprints/Saant_Sve_BP.SaveData` :`self` _output_get :`CurrentLevel` "GameplayMap" :`Current_Position` (-1683.0 -975.0 176.0) :`Difficulty` (`self.Difficulty`))
    (else
      (bind (_ar_ammo_current _shotgun_ammo_current _health _currentlevel _current_position _current_rotation) (`/Game/Blueprints/Saant_Sve_BP.SetData` _output_get))
      (`/Game/Blueprints/Saant_Sve_BP.SaveData` _output_get _ar_ammo_current _shotgun_ammo_current _health _currentlevel _current_position _current_rotation (`self.Difficulty`))))
  (`GameplayStatics.SaveGameToSlot` _output_get (`self.SaveName`))
  (return))

(fn `UserConstructionScript`)
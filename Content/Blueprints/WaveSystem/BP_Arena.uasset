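; BP_Arena is a wave-system arena actor that closes the entrance behind the player and animates the exit when the arena ends.
; A one-time TriggerIn overlap by BP_SaantCharacter calls StartArena, which moves the entrance spikes and stairs, then enables BlockingIn collision.
; EndArena, not called within this Blueprint, moves the exit spikes and stairs.
; Both timelines add fixed Z offsets per update, so travel distance depends on frame rate.
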(event `self.TriggerIn.OnComponentBeginOverlap`
  (params (OverlappedComponent :type "PrimitiveComponent Object Reference") (OtherActor :type "Actor Object Reference") (OtherComp :type "PrimitiveComponent Object Reference") (OtherBodyIndex :type Integer) (bFromSweep :type Boolean) (SweepResult :type "HitResult Structure (by ref)"))
  (`/Engine/EditorBlueprintResources/StandardMacros.DoOnce` false
    (:`Completed`
      (cast `/Game/Blueprints/Character/BP_SaantCharacter` OtherActor)
      (`self.StartArena`)
      (`PrimitiveComponent.SetCollisionEnabled` (`self.BlockingIn`) "QueryAndPhysics"))))

(event `StartArena`
  (`Timeline|StairsIn`
    (:`Update`
      (`SceneComponent.K2_AddRelativeLocation` (`self.SpikeStairsIn`) (0.0 0.0 -3.0) false false)
      (`SceneComponent.K2_AddRelativeLocation` (`self.SpikesOpenIn`) (0.0 0.0 3.35) false false))))

(event `/Game/Blueprints/WaveSystem/BPI_Arena.EndArena`
  (`Timeline|Timeline`
    (:`Update`
      (`SceneComponent.K2_AddRelativeLocation` (`self.SpikesOpenOut`) (0.0 0.0 -4.0) false false)
      (`SceneComponent.K2_AddRelativeLocation` (`self.SpikeStairsOut`) (0.0 0.0 3.0) false false))))

(fn `UserConstructionScript`)
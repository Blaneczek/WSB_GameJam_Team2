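; BP_Turret is an enemy turret that attacks by firing a BP_SaantProjectile at the player character.
; The Attack event spawns the projectile at the ProjectileSpawn component, rotated along the look-at direction from the turret's actor location to the player's.
; SetMovementSpeed ignores its input and always returns zero, and the construction script only calls its parent.
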(event `Attack`
  (`|SpawnActorFromClass` "/Game/Blueprints/BP_SaantProjectile.BP_SaantProjectile_C" (`KismetMathLibrary.MakeTransform` (`SceneComponent.K2_GetComponentLocation` (`self.ProjectileSpawn`)) (`KismetMathLibrary.FindLookAtRotation` (`self.K2_GetActorLocation`) (`self.K2_GetActorLocation` (`GameplayStatics.GetPlayerCharacter` 0)))) "Undefined" "MultiplyWithRoot" null null))

(fn `SetMovementSpeed`
  (params (Speed :type "/Game/AI/Enums/EMovementSpeed Enum" :default "NewEnumerator0"))
  (returns (SpeedValue :type "Float (double-precision)"))
  (return 0.0))

(fn `UserConstructionScript`
  (`parent.UserConstructionScript`))
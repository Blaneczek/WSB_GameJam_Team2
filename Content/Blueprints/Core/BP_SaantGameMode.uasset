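; BP_SaantGameMode is a game mode that sets up the player HUD and tracks combat state and battle music.
; On BeginPlay it creates and displays Player_UI, while PlayBattleMusic starts a stored 2D track unless enemies are dead.
; During a fight, Tick watches AliveEnemies, ending combat and stopping the music after a short delay at zero.
; EnemiesLeft separately checks EnemiesAlive and triggers CallSpawnEnemy when it reaches zero.
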(event `self.ReceiveBeginPlay`
  (bind _returnvalue (`|CreateWidget` "/Game/UI/Player_UI.Player_UI_C"))
  (set `self.Player_UI_Ref` _returnvalue)
  (`UserWidget.AddToViewport` _returnvalue 0))

(event `PlayBattleMusic`
  (if (not (`self.EnemiesDead`))
    (bind _returnvalue (`GameplayStatics.SpawnSound2D` "/Game/Music/All_I_Want_For_Christmas_Is_DOOM_v_2__BFG_Division_x_AIWFCIY_-YConverter_app.All_I_Want_For_Christmas_Is_DOOM_v_2__BFG_Division_x_AIWFCIY_-YConverter_app" 1.0 1.0 0.0 null))
    (set `self.2DSound` _returnvalue)))

(event `self.ReceiveTick`
  (params (DeltaSeconds :type "Float (single-precision)"))
  (bind _2dsound (`self.2DSound`))
  (if (`self.Fighting?`)
    (if (== (`self.AliveEnemies`) 0)
      (set `self.EnemiesDead` true)
      (set `self.Fighting?` false)
      (`/Engine/EditorBlueprintResources/StandardMacros.IsValid` _2dsound
        (:`Is Valid`
          (`AudioComponent.StopDelayed` _2dsound 1.0))))))

(event `EnemiesLeft`
  (if (== (`self.EnemiesAlive`) 0)
    (`self.SpawnEnemy`)))

(fn `UserConstructionScript`)